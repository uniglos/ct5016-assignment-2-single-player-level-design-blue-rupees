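; BP_LevenEndCheck is a level actor that toggles the visibility of a set of enemies and dialogue triggers, apparently for the level's end.
; On BeginPlay it hides both groups through the Enableorhidelevelend event, which can also reveal them when called with false.
; The event loops over both actor arrays, skipping invalid entries, and sets only Hidden In Game, leaving collision and tick untouched.
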(event Custom|enableorhidelevelend
  (params (bNewHidden :type Boolean))
  (Utilities|FlowControl|Sequence
    (:then_0
      (for _array_element (Variables|Components|GetEneimes)
        (Utilities|IsValid _array_element
          (:Is%20Valid
            (Rendering|SetActorHiddenInGame _array_element bNewHidden))
          (:Is%20Not%20Valid
            (Development|PrintString "Hello")))))
    (:then_1
      (for _array_element_2 (Variables|Default|GetDialougeTriggers)
        (Utilities|IsValid _array_element_2
          (:Is%20Valid
            (Rendering|SetActorHiddenInGame _array_element_2 bNewHidden)))))))

(event EventBeginPlay
  (CallFunction|Enableorhidelevelend true))

(event Collision|EventActorBeginOverlap
  (params (OtherActor :type Actor%20Object%20Reference)))

(event EventTick
  (params (DeltaSeconds :type Float%20%28single-precision%29)))

(fn ConstructionScript)