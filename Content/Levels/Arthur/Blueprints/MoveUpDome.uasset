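; MoveUpDome is a level Blueprint actor that animates a dome opening when its OpenNEWDOME event fires.
; A timeline drives the relative Z location of eleven "Er" components together, scaling its track by -2.
; When the timeline finishes, the actor destroys itself.
; The OpenDoor and NewFunction functions are empty.
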(event Custom|OpenNEWDOME
  (bind _newtrack_0 (Timeline|Timeline Play)
    (:Update
      (Transformation|SetRelativeLocation (Variables|Components|Geter) (Math|Vector|MakeVector 0.0 0.0 (* _newtrack_0 -2.0)) false false))
    (:Finished
      (Actor|DestroyActor))))

(event Collision|EventActorBeginOverlap
  (params (OtherActor :type Actor%20Object%20Reference)))

(event EventTick
  (params (DeltaSeconds :type Float%20%28single-precision%29)))

(fn ConstructionScript)

(fn OpenDoor)

(fn NewFunction)