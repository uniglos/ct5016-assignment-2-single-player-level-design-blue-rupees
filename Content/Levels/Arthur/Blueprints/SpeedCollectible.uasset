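; A spinning speed pickup that permanently boosts the walk speed of a BP_Player_Test_Gravity player who touches it.
; A looping timer calls Rotate to tumble the root component slightly on each tick.
; Box overlap sets the player's MaxWalkSpeed to a huge multiple of its current GetMaxSpeed, then destroys the pickup.
; The SpeedBoostOn flag and its delayed reset are unconnected, so the boost never expires here.
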(event OnComponentBeginOverlap(Box)
  (params (OverlappedComponent :type Primitive%20Component%20Object%20Reference) (OtherActor :type Actor%20Object%20Reference) (OtherComp :type Primitive%20Component%20Object%20Reference) (OtherBodyIndex :type Integer) (bFromSweep :type Boolean) (SweepResult :type Hit%20Result%20Structure%20%28by%20ref%29))
  (bind _asbp_player_test_gravity (Utilities|Casting|CastToBP_Player_Test_Gravity OtherActor))
  (Variables|/Script/Engine.CharacterMovementComponent|SetMaxWalkSpeed (Actor|GetComponentbyClass _asbp_player_test_gravity "/Script/Engine.CharacterMovementComponent") (* (Class|MovementComponent|GetMaxSpeed (Actor|GetComponentbyClass _asbp_player_test_gravity "/Script/Engine.CharacterMovementComponent")) 99.0))
  (Actor|DestroyActor))

(event EventBeginPlay
  (Utilities|Time|SetTimerbyFunctionName 0 "Rotate" 0.008 true))

(fn ConstructionScript)

(fn Rotate
  (Transformation|AddLocalRotation (Variables|Default|GetDefaultSceneRoot) (Math|Rotator|MakeRotator 0.2 0.3 0.5) false false))