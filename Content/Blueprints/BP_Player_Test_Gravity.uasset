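; Test player character with an airborne hover and a pickup goal that opens a dome.
; Each Tick, holding E while off the ground slightly lowers gravity scale and pins vertical velocity to a small upward value, otherwise restoring normal gravity.
; Tick also calls OpenNEWDOME on the MoveUpDome reference stored at BeginPlay whenever PickupCount equals OverallCount.
; Destruction of the character opens the OceanWorking level.
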(event EventBeginPlay
  (|CallParentFunction)
  (Variables|Default|SetMove%20Up%20Dome%20Ref "/Game/Levels/Arthur/Blueprints/MoveUpDome.MoveUpDome"))

(event Collision|EventActorBeginOverlap
  (params (OtherActor :type Actor%20Object%20Reference)))

(event EventTick
  (params (DeltaSeconds :type Float%20%28single-precision%29))
  (bind _charactermovement (Variables|Character|GetCharacterMovement))
  (Utilities|FlowControl|Sequence
    (:then_0
      (|CallParentFunction DeltaSeconds))
    (:then_1
      (if (Game|Player|IsInputKeyDown (Game|GetPlayerController 0) "E")
        (if (AI|Components|NavMovement|IsMovingonGround (Variables|Character|GetCharacterMovement))
          (Variables|/Script/Engine.CharacterMovementComponent|SetGravityScale (Variables|Character|GetCharacterMovement) 1.0 :!label _label)
          (else
            (Variables|/Script/Engine.CharacterMovementComponent|SetGravityScale _charactermovement 0.9)
            (Variables|/Script/Engine.MovementComponent|SetVelocity _charactermovement (Math|Vector|MakeVector (.x (Variables|/Script/Engine.MovementComponent|GetVelocity _charactermovement)) (.y (Variables|/Script/Engine.MovementComponent|GetVelocity _charactermovement)) 9.0))))
        (else
          (goto _label))))
    (:then_2
      (if (== (Variables|Default|GetPickup%20Count) (Variables|Default|GetOverall%20Count))
        (bind _asmove_up_dome (Utilities|Casting|CastToMoveUpDome (Variables|Default|GetMove%20Up%20Dome%20Ref)))
        (Default|OpenNEWDOME _asmove_up_dome)))))

(event EventDestroyed
  (Game|OpenLevel(byName) "OceanWorking"))

(fn ConstructionScript
  (|CallParentFunction))