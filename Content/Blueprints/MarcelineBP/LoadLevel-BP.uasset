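; A level portal Blueprint that loads a named level when the player walks into its box trigger.
; On BeginPlay it sets its text label from the level name.
; On overlap it casts to BP_Player, prints a debug message and opens the level, requiring the player to have a key when NeedsKey is set.
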(event OnComponentBeginOverlap(Box)
  (params (OverlappedComponent :type Primitive%20Component%20Object%20Reference) (OtherActor :type Actor%20Object%20Reference) (OtherComp :type Primitive%20Component%20Object%20Reference) (OtherBodyIndex :type Integer) (bFromSweep :type Boolean) (SweepResult :type Hit%20Result%20Structure%20%28by%20ref%29))
  ;[1 1 1] when the player collides with this box load new level
  (bind _asbp_player (Utilities|Casting|CastToBP_Player OtherActor))
  (Development|PrintString "player was hit")
  (if (Variables|Default|GetneedsKey?)
    (if (Variables|/Game/Blueprints/BP_Player.BP_Player_C|GethasKey _asbp_player)
      (Game|OpenLevel(byName) (Variables|Default|GetLevel%20Name) :!label _label))
    (else
      (goto _label))))

(event EventBeginPlay
  ;[1 1 1] this makes sure our level text is the same as our level name when we oopen it
  (Rendering|Components|TextRender|SetText (Variables|Default|GetLevelText) (Utilities|Text|ToText(String) (Utilities|String|Append (Variables|Default|GetA) (Utilities|String|ToString(Name) (Variables|Default|GetLevel%20Name))))))

(fn ConstructionScript)