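; BP_endLevel is a level-end trigger that checks whether the player has collected every BP_File in the level.
; BeginPlay caches the player and the file count, and computes a spawn point just above the BP_BoatV2 mesh.
; Each Tick, a full collection plays the all-files audio once and spawns a BP_LoadLevel at the boat with its level name and text.
; Otherwise, overlapping PlayerCollisonZone triggers a one-time missing-files line.
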(event OnComponentBeginOverlap(PlayerCollisonZone)
  (params (OverlappedComponent :type Primitive%20Component%20Object%20Reference) (OtherActor :type Actor%20Object%20Reference) (OtherComp :type Primitive%20Component%20Object%20Reference) (OtherBodyIndex :type Integer) (bFromSweep :type Boolean) (SweepResult :type Hit%20Result%20Structure%20%28by%20ref%29))
  (bind _asbp_player_test_gravity (Utilities|Casting|CastToBP_Player_Test_Gravity OtherActor))
  (Variables|Default|SetplayerHasReachedObTower true)
  (Variables|Default|SetPlayer _asbp_player_test_gravity))

(event Custom|set%20and%20play%20audio
  (params (NewSound :type Sound%20Base%20Object%20Reference))
  (bind _dialougesource (Variables|Default|GetDialougeSource))
  ;[1 1 1] sets our dialouge for audio and plays it
  (Audio|Components|Audio|SetSound _dialougesource NewSound)
  (Audio|Components|Audio|Play _dialougesource 0.0))

(event Custom|spawnLevelEndActors
  ;[1 1 1] spawn end levels
  (bind _returnvalue (Game|SpawnActorfromClass "/Game/Blueprints/MarcelineBP/BP_LoadLevel.BP_LoadLevel_C" (Variables|Default|GetSpawn%20Transform) "Undefined" "MultiplyWithRoot" 0 "None" 0))
  (Variables|/Game/Blueprints/MarcelineBP/BP_LoadLevel.BP_LoadLevel_C|SetLevel%20Name _returnvalue (Variables|Default|GetLevel%20Name))
  (Rendering|Components|TextRender|SetText (Variables|/Game/Blueprints/MarcelineBP/BP_LoadLevel.BP_LoadLevel_C|GetLevelText _returnvalue) (Variables|Default|GetValue)))

(event EventBeginPlay
  ;[1 1 1] get player
  (bind _outactors (Actor|GetAllActorsOfClass "/Game/Blueprints/BP_Player_Test_Gravity.BP_Player_Test_Gravity_C"))
  (Variables|Default|SetPlayerBP (Utilities|Array|Get(acopy) _outactors))
  (bind _outactors_2 (Actor|GetAllActorsOfClass "/Game/Blueprints/MarcelineBP/BP_File.BP_File_C"))
  (Variables|Default|Setfiletotal (Utilities|Array|Length _outactors_2))
  (bind _outactors_3 (Actor|GetAllActorsOfClass "/Game/Blueprints/MarcelineBP/BP_BoatV2.BP_BoatV2_C"))
  (Variables|Default|SetSpawn%20Transform (Math|Transform|MakeTransform (Math|Vector|MakeVector (.x (Transformation|GetWorldLocation (Variables|/Game/Blueprints/MarcelineBP/BP_BoatV2.BP_BoatV2_C|GetBoatMesh (Utilities|Array|Get(acopy) _outactors_3)))) (.y (Transformation|GetWorldLocation (Variables|/Game/Blueprints/MarcelineBP/BP_BoatV2.BP_BoatV2_C|GetBoatMesh (Utilities|Array|Get(acopy) _outactors_3)))) (+ (.z (Transformation|GetWorldLocation (Variables|/Game/Blueprints/MarcelineBP/BP_BoatV2.BP_BoatV2_C|GetBoatMesh (Utilities|Array|Get(acopy) _outactors_3)))) 3e+01)) "0, 0, 0" "1.000000,1.000000,1.000000")))

(event EventTick
  (params (DeltaSeconds :type Float%20%28single-precision%29))
  ;[1 1 1] if player is valid and end level bp
  (Utilities|FlowControl|Sequence
    (:then_0
      (Utilities|IsValid (Variables|Default|GetPlayerBP)
        (:Is%20Valid
          (if (== (Variables|/Game/Blueprints/BP_Player.BP_Player_C|GetFilesCollected (Variables|Default|GetPlayerBP)) (Variables|Default|Getfiletotal))
            ;[1 1 1] then we set and play are audio on a DO ONCE NODE SO IT WONT REPEAT
            ;;[1 1 1] have all files play all file dialouge
            (Utilities|FlowControl|DoOnce false
              (:Completed
                (CallFunction|SetandPlayAudio (Variables|Default|GetGameEndAudioAllFiles))
                (CallFunction|SpawnLevelEndActors)))
            (elif (== (Variables|Default|GetplayerHasReachedObTower) true)
              ;;[1 1 1] play missing file dialouge
              (Utilities|FlowControl|DoOnce false
                (:Completed
                  (CallFunction|SetandPlayAudio (Variables|Default|GetGameEndAudioMissingFiles)))))))))))

(fn ConstructionScript)