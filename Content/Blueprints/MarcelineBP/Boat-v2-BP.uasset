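; Boat actor Blueprint that shows a button hint widget when a player enters its PlayerOnBoat overlap component.
; On begin overlap, it stores the BP_Player if that player has no valid Boat, then adds a WD_BoatButtonHint to the viewport, creating it once and reusing it.
; On end overlap by a player, it removes the hint; no boarding or movement logic is in this graph.
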(event OnComponentBeginOverlap(PlayerOnBoat)
  (params (OverlappedComponent :type Primitive%20Component%20Object%20Reference) (OtherActor :type Actor%20Object%20Reference) (OtherComp :type Primitive%20Component%20Object%20Reference) (OtherBodyIndex :type Integer) (bFromSweep :type Boolean) (SweepResult :type Hit%20Result%20Structure%20%28by%20ref%29))
  (bind _asbp_player (Utilities|Casting|CastToBP_Player OtherActor))
  (Utilities|IsValid (Variables|/Game/Blueprints/BP_Player.BP_Player_C|GetBoat _asbp_player)
    (:Is%20Not%20Valid
      (Variables|Default|SetAs%20BP%20Player _asbp_player)
      (Utilities|IsValid (Variables|Default|GetNewVar)
        (:Is%20Valid
          (UserInterface|Viewport|AddtoViewport (Variables|Default|GetNewVar) 0))
        (:Is%20Not%20Valid
          (bind _returnvalue (UserInterface|CreateWidget "/Game/UI/MarcelineWidgets/WD_BoatButtonHint.WD_BoatButtonHint_C"))
          (bind _output_get (Variables|Default|SetNewVar _returnvalue))
          (UserInterface|Viewport|AddtoViewport _output_get 0))))))

(event OnComponentEndOverlap(PlayerOnBoat)
  (params (OverlappedComponent :type Primitive%20Component%20Object%20Reference) (OtherActor :type Actor%20Object%20Reference) (OtherComp :type Primitive%20Component%20Object%20Reference) (OtherBodyIndex :type Integer))
  (Utilities|Casting|CastToBP_Player OtherActor)
  (Widget|RemovefromParent (Variables|Default|GetNewVar)))

(fn ConstructionScript)