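; TV actor that acts as a portal, teleporting the player to the location of a linked camera.
; At construction, it assigns a render target to its scene capture component and moves that component to the linked Camera's location and rotation.
; When BP_Player overlaps the box collision, it teleports to the scene capture's position and rotation, so the capture viewpoint doubles as the destination.
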(event OnComponentBeginOverlap(BoxCollison)
  (params (OverlappedComponent :type Primitive%20Component%20Object%20Reference) (OtherActor :type Actor%20Object%20Reference) (OtherComp :type Primitive%20Component%20Object%20Reference) (OtherBodyIndex :type Integer) (bFromSweep :type Boolean) (SweepResult :type Hit%20Result%20Structure%20%28by%20ref%29))
  (bind _scenecapturecomponent2d (Variables|Default|GetSceneCaptureComponent2D))
  ;[1 1 1] teleport player on overlap
  (bind _asbp_player (Utilities|Casting|CastToBP_Player OtherActor))
  (Transformation|Teleport _asbp_player (Transformation|GetWorldLocation _scenecapturecomponent2d) (Transformation|GetWorldRotation _scenecapturecomponent2d)))

(event EventBeginPlay)

(event Collision|EventActorBeginOverlap
  (params (OtherActor :type Actor%20Object%20Reference)))

(event EventTick
  (params (DeltaSeconds :type Float%20%28single-precision%29)))

(fn ConstructionScript
  (bind _scenecapturecomponent2d (Variables|Default|GetSceneCaptureComponent2D))
  (bind _camera (Variables|Default|GetCamera))
  ;[1 1 1] once we add our scence camera set it to the texture target
  (Utilities|IsValid (Variables|Default|GetSceneCaptureComponent2D)
    (:Is%20Valid
      (Variables|/Script/Engine.SceneCaptureComponent2D|SetTextureTarget _scenecapturecomponent2d (Variables|Default|GetTexture%20Target))
      (Transformation|SetWorldLocation _scenecapturecomponent2d (Transformation|GetWorldLocation (Variables|/Script/Engine.Actor|GetRootComponent _camera)) false false)
      (Transformation|SetWorldRotation (Variables|Default|GetSceneCaptureComponent2D) (Transformation|GetWorldRotation (Variables|/Script/Engine.CameraActor|GetCameraComponent _camera)) false false))))

(fn NewFunction)