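; BP_File is a collectible audio file that adds to the player's FilesCollected count once its audio has played.
; BeginPlay stops the audio and caches the first BP_Player actor.
; The first player overlap with the Box starts playback and arms a Tick poll.
; When playback ends, Tick sets Hasplayed, then on a later tick adds FilesGained to the player and destroys the actor.
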(event OnComponentBeginOverlap(Box)
  (params (OverlappedComponent :type Primitive%20Component%20Object%20Reference) (OtherActor :type Actor%20Object%20Reference) (OtherComp :type Primitive%20Component%20Object%20Reference) (OtherBodyIndex :type Integer) (bFromSweep :type Boolean) (SweepResult :type Hit%20Result%20Structure%20%28by%20ref%29))
  ;[1 1 1] play audio only once
  (Utilities|Casting|CastToBP_Player OtherActor)
  (Utilities|FlowControl|DoOnce false
    (:Completed
      (Audio|Components|Audio|Play (Variables|Default|GetAudio) 0.0)
      ;;[1 1 1] player has entered needs to be true so event tick code only runs based on the object
      (Variables|Default|SetPlayerHasEntered true))))

(event EventBeginPlay
  ;[1 1 1] start play
  (Audio|Components|Audio|Stop (Variables|Default|GetAudio))
  (bind _outactors (Actor|GetAllActorsOfClass "/Game/Blueprints/BP_Player.BP_Player_C"))
  (Variables|Default|Setplayer (Utilities|Array|Get(acopy) _outactors)))

(event EventTick
  (params (DeltaSeconds :type Float%20%28single-precision%29))
  ;[1 1 1] when audio is not playing we will run this code
  (if (Variables|Default|GetPlayerHasEntered)
    (if (Variables|Default|Gethasplayed)
      (if (not (Audio|Components|Audio|IsPlaying (Variables|Default|GetAudio)))
        (Utilities|IsValid (Variables|Default|Getplayer)
          (:Is%20Valid
            (Utilities|FlowControl|DoOnce false
              (:Completed
                (Variables|/Game/Blueprints/BP_Player.BP_Player_C|SetFilesCollected (Variables|Default|Getplayer) (+ (Variables|/Game/Blueprints/BP_Player.BP_Player_C|GetFilesCollected (Variables|Default|Getplayer)) (Variables|Default|GetfilesGained)))
                (Actor|DestroyActor))))))
      (elif (not (Audio|Components|Audio|IsPlaying (Variables|Default|GetAudio)))
        (Variables|Default|Sethasplayed true)))))

(fn ConstructionScript)