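; Dialogue trigger actor that plays a voice line through its Audio component, either automatically or when the player enters its box.
; On BeginPlay it plays at once if Autplay is set, otherwise it stops the audio.
; A BP_Player overlap plays the audio once, guarded by Hasplayed.
; When the player leaves the box after playback has started, the actor destroys itself.
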(event OnComponentBeginOverlap(Box)
  (params (OverlappedComponent :type Primitive%20Component%20Object%20Reference) (OtherActor :type Actor%20Object%20Reference) (OtherComp :type Primitive%20Component%20Object%20Reference) (OtherBodyIndex :type Integer) (bFromSweep :type Boolean) (SweepResult :type Hit%20Result%20Structure%20%28by%20ref%29))
  ;[1 1 1] player overlaps with trigger start dialouge
  (Utilities|Casting|CastToBP_Player OtherActor)
  (if (not (Variables|Default|Gethasplayed))
    (Audio|Components|Audio|Play (Variables|Default|GetAudio) 0.0)
    (Variables|Default|Sethasplayed true)))

(event OnComponentEndOverlap(Box)
  (params (OverlappedComponent :type Primitive%20Component%20Object%20Reference) (OtherActor :type Actor%20Object%20Reference) (OtherComp :type Primitive%20Component%20Object%20Reference) (OtherBodyIndex :type Integer))
  ;[1 1 1] destroy actor when we leave and played are dialouge
  (Utilities|Casting|CastToBP_Player OtherActor)
  (if (Variables|Default|Gethasplayed)
    (Actor|DestroyActor)))

(event EventBeginPlay
  ;[1 1 1] if has play is true auto play dialouge
  (if (Variables|Default|Getautplay)
    (Audio|Components|Audio|Play (Variables|Default|GetAudio) 0.0)
    (Variables|Default|Sethasplayed true)
    (else
      (Audio|Components|Audio|Stop (Variables|Default|GetAudio)))))

(event Collision|EventActorBeginOverlap
  (params (OtherActor :type Actor%20Object%20Reference)))

(event EventTick
  (params (DeltaSeconds :type Float%20%28single-precision%29))
  ;[1 1 1] player overlaps with trigger start dialouge
)

(fn ConstructionScript)