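; Drivable boat pawn that the player can board, steer and leave.
; An overlap zone flags BP_Player as within range and shows a button hint widget.
; Boarding teleports the player to a dummy seat position, blends the view to the boat, and switches input and possession to it.
; Enhanced Input drives movement along control-yaw axes, while the step action unpossesses the boat, re-enables player input and blends back to the ALS camera manager.
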(event OnComponentBeginOverlap(BoatOverLap)
  (params (OverlappedComponent :type Primitive%20Component%20Object%20Reference) (OtherActor :type Actor%20Object%20Reference) (OtherComp :type Primitive%20Component%20Object%20Reference) (OtherBodyIndex :type Integer) (bFromSweep :type Boolean) (SweepResult :type Hit%20Result%20Structure%20%28by%20ref%29))
  ;[1 1 1] player entered boat collision zone
  (bind _asbp_player (Utilities|Casting|CastToBP_Player OtherActor))
  (Variables|Default|SetAs%20BP%20Player _asbp_player)
  (Variables|/Game/Blueprints/BP_Player.BP_Player_C|SetPlayerWithinBoatZone (Variables|Default|GetAs%20BP%20Player) true)
  (Utilities|IsValid (Variables|Default|GetCurrentBoatHint)
    (:Is%20Valid
      (UserInterface|Viewport|AddtoViewport (Variables|Default|GetCurrentBoatHint) 0))
    (:Is%20Not%20Valid
      (bind _returnvalue (UserInterface|CreateWidget "/Game/UI/MarcelineWidgets/WD_BoatButtonHint.WD_BoatButtonHint_C"))
      (Variables|Default|SetCurrentBoatHint _returnvalue)
      (UserInterface|Viewport|AddtoViewport (Variables|Default|GetCurrentBoatHint) 0))))

(event OnComponentEndOverlap(BoatOverLap)
  (params (OverlappedComponent :type Primitive%20Component%20Object%20Reference) (OtherActor :type Actor%20Object%20Reference) (OtherComp :type Primitive%20Component%20Object%20Reference) (OtherBodyIndex :type Integer))
  ;[1 1 1] player out of overlap zone
  (Utilities|Casting|CastToBP_Player OtherActor)
  (Variables|/Game/Blueprints/BP_Player.BP_Player_C|SetPlayerWithinBoatZone (Variables|Default|GetAs%20BP%20Player) false)
  (Utilities|IsValid (Variables|Default|GetCurrentBoatHint)
    (:Is%20Valid
      (Widget|RemovefromParent (Variables|Default|GetCurrentBoatHint)))))

(event Custom|C_GetOntoBoat
  ;[1 1 1] get on boat
  (Transformation|Teleport (Variables|Default|GetAs%20BP%20Player) (Transformation|GetWorldLocation (Variables|Default|GetDummyPlayer)) "0, 0, 0")
  (Utilities|FlowControl|Delay 0.2)
  (Game|Player|SetViewTargetwithBlend (Game|GetPlayerController 0) self 0.0 "VTBlend_Cubic" 0.0 false)
  (Widget|RemovefromParent (Variables|Default|GetCurrentBoatHint))
  (Input|DisableInput (Variables|Default|GetAs%20BP%20Player) (Game|GetPlayerController 0))
  (Input|EnableInput self (Game|GetPlayerController 0))
  (Pawn|Possess (Game|GetPlayerController 0) self)
  (bind _asplayer_controller (Utilities|Casting|CastToPlayerController (Pawn|GetController)))
  (bind _output_get (Variables|Default|SetAs%20Player%20Controller _asplayer_controller))
  (Input|AddMappingContext (PlayerController|LocalPlayerSubsystems|GetEnhancedInputLocalPlayerSubsystem _output_get) "/Game/Blueprints/MarcelineBP/Input/3rdPersonPlayer_Context.3rdPersonPlayer_Context" 0 "(bIgnoreAllPressedKeysUntilRelease=True,bForceImmediately=False,bNotifyUserSettings=False)"))

(event Custom|boat_Movement_fwp
  (params (ScaleValue :type Float%20%28single-precision%29) (bForce :type Boolean))
  ;[1 1 1] boat forward movement
  (Pawn|Input|AddMovementInput (Math|Vector|GetForwardVector (Math|Rotator|MakeRotator 0.0 0.0 (.yaw (Pawn|GetControlRotation :!class /Script/Engine.Pawn)))) ScaleValue bForce))

(event Custom|boat_Movement_right
  (params (ScaleValue :type Float%20%28single-precision%29) (bForce :type Boolean))
  (bind _returnvalue (Pawn|GetControlRotation :!class /Script/Engine.Pawn))
  ;[1 1 1] boat right movement
  (Pawn|Input|AddMovementInput (Math|Vector|GetRightVector (Math|Rotator|MakeRotator (.roll _returnvalue) 0.0 (.yaw _returnvalue))) ScaleValue bForce))

(event Input|EnhancedActionEvents|EnhancedInputActionIA_StepOnBoat
  (params (ActionValue :type Boolean) (ElapsedSeconds :type Float%20%28double-precision%29) (TriggeredSeconds :type Float%20%28double-precision%29) (InputAction :type Input%20Action%20Object%20Reference :default "/Game/Blueprints/MarcelineBP/Input/IA_StepOnBoat.IA_StepOnBoat"))
  ;[1 1 1] step on boat
  (Development|PrintString "hi")
  (Input|DisableInput (Game|GetPlayerController 0))
  (Input|EnableInput (Variables|Default|GetAs%20BP%20Player) (Game|GetPlayerController 0))
  (Pawn|UnPossess (Game|GetPlayerController 0))
  (Game|Player|SetViewTargetwithBlend (Game|GetPlayerController 0) (Variables|Default|GetALSPlayerCameraManger) 0.0 "VTBlend_Cubic" 0.0 false))

(event Input|EnhancedActionEvents|EnhancedInputActionIA_BoatMove
  (params (ActionValue :type Vector%202D%20Structure) (ElapsedSeconds :type Float%20%28double-precision%29) (TriggeredSeconds :type Float%20%28double-precision%29) (InputAction :type Input%20Action%20Object%20Reference :default "/Game/Blueprints/MarcelineBP/Input/IA_BoatMove.IA_BoatMove"))
  ;[1 1 1] boat input action
  (CallFunction|BoatMovementRight (.x ActionValue) true)
  (CallFunction|BoatMovementFwp (.y ActionValue) true)
  (Development|PrintString "Hello"))

(event EventBeginPlay
  ;[1 1 1] begin play zone
  (bind _outactors (Actor|GetAllActorsOfClass "/Game/AdvancedLocomotionV4/Blueprints/CameraSystem/ALS_PlayerCameraManager.ALS_PlayerCameraManager_C"))
  (Variables|Default|SetALSPlayerCameraManger (Utilities|Array|Get(acopy) _outactors))
  (Input|AddMappingContext (PlayerController|LocalPlayerSubsystems|GetEnhancedInputLocalPlayerSubsystem 0) "/Game/Blueprints/MarcelineBP/Input/3rdPersonPlayer_Context.3rdPersonPlayer_Context" 0 "(bIgnoreAllPressedKeysUntilRelease=True,bForceImmediately=False,bNotifyUserSettings=False)"))

(fn ConstructionScript)